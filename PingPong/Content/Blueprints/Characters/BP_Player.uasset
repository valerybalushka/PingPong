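; BP_Player is the player Blueprint that holds, aims and launches a ball.
; SetupBall attaches the ball to BallHolder, pauses its tick, shows its arrow and starts a timeline that drives its yaw relative to the player's rotation.
; LaunchBall runs on authority, routed through a server event from remotes, to stop aiming, detach and restart the ball, then clear the reference.
; The camera detaches at BeginPlay, keeping its world transform.
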(event `self.ReceiveBeginPlay`
  (`SceneComponent.K2_DetachFromComponent` (`self.Camera`) "KeepWorld" "KeepWorld" "KeepWorld" true))

(event `StartSelectDirection`
  (bind (_direction _balldirection) (`Timeline|Timeline_BallDirection`)
    (:`Update`
      (bind _ball (`self.Ball`)
        (:`then`
          (`self.K2_SetActorRotation` _ball (`KismetMathLibrary.MakeRotator` 0.0 0.0 (+ _balldirection (.yaw (`self.K2_GetActorRotation`)))) false))
        (:`else`)))))

(event `self.LaunchBall`
  (`self.Ball`
    (:`then`
      (`/Engine/EditorBlueprintResources/ActorMacros.Switch Has Authority`
        (:`Authority`
          (`TimelineComponent.Stop` (`self.Timeline_BallDirection`))
          (`self.K2_DetachFromActor` (`self.Ball`) "KeepWorld" "KeepWorld" "KeepWorld")
          (`PingPongBall.RestartBallSpeed` (`self.Ball`))
          (bind _ball (`self.Ball`)
            (:`then`
              (`/Game/Blueprints/Actors/BP_Ball.SetArrowHiddenInGame` _ball true)
              (`self.SetActorTickEnabled` (`self.Ball`) true)
              (set `self.Ball` null))
            (:`else`)))
        (:`Remote`
          (`self.LaunchBall_Server`))))
    (:`else`)))

(event `LaunchBall_Server`
  (`self.LaunchBall`))

(event `self.SetupBall`
  (params (Ball :type "PingPongBall Object Reference"))
  (bind _asbp_ball (cast `/Game/Blueprints/Actors/BP_Ball` Ball))
  (bind _output_get (set `self.Ball` _asbp_ball))
  (`self.SetActorTickEnabled` _output_get false)
  (`self.K2_AttachToComponent` (`self.Ball`) (`self.BallHolder`) "None" "SnapToTarget" "SnapToTarget" "KeepWorld" true)
  (`/Game/Blueprints/Actors/BP_Ball.SetArrowHiddenInGame` (`self.Ball`) false)
  (`self.StartSelectDirection`))

(fn `OnRep_Ball`)

(fn `UserConstructionScript`)